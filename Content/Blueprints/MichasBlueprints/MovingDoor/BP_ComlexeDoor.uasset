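; BP_ComlexeDoor is a moving door that slides a static mesh along a spline while its StartFirstMove event reports pressed, and returns it on release.
; Tick plays or reverses the MoveDoor timeline, with play rates derived from separate up and down durations.
; The Open flag inverts the direction and starts the timeline at its end.
; Non-Open doors wait before lowering from the top, detected by comparing relative Z to spline length.
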(event `StartFirstMove`
  (params (Pressed :type Boolean))
  (set `self.Start Move` Pressed))

(event `self.ReceiveTick`
  (params (DeltaSeconds :type "Float (single-precision)"))
  (bind _returnvalue (`SplineComponent.GetSplineLength` (`self.Spline`)))
  (bind (_relativelocation_x _relativelocation_y _relativelocation_z) (`KismetMathLibrary.BreakVector` (`SceneComponent.RelativeLocation` (`self.StaticMesh`))))
  (bind (_relativelocation_x_2 _relativelocation_y_2 _relativelocation_z_2) (`KismetMathLibrary.BreakVector` (`SceneComponent.RelativeLocation` (`self.StaticMesh`))))
  (if (not (`self.Open`))
    (if (`self.Start Move`)
      (`TimelineComponent.SetPlayRate` (`self.MoveDoor`) (/ 1.0 (`self.UpMovingTime`)))
      (bind (_direction _newtrack_0) (`Timeline|MoveDoor` :!label _label)
        (:`Update`
          (`SceneComponent.K2_SetWorldLocation` (`self.StaticMesh`) (`SplineComponent.GetLocationAtDistanceAlongSpline` (`self.Spline`) (* _newtrack_0 (`SplineComponent.GetSplineLength` (`self.Spline`))) "World") false false)))
      (elif (<= (- (`SplineComponent.GetSplineLength` (`self.Spline`)) 1.0) _relativelocation_z_2)
        (`TimelineComponent.SetPlayRate` (`self.MoveDoor`) (/ 1.0 (`self.DownMovingTime`)))
        (`KismetSystemLibrary.Delay` (`self.WaitingTime`))
        (goto _label :!via `Reverse`)
        (else
          (goto _label :!via `Reverse`))))
    (elif (`self.Start Move`)
      (`TimelineComponent.SetPlayRate` (`self.MoveDoor`) (/ 1.0 (`self.DownMovingTime`)))
      (goto _label :!via `Reverse`)
      (elif (<= _relativelocation_z (- _returnvalue _returnvalue))
        (`TimelineComponent.SetPlayRate` (`self.MoveDoor`) (/ 1.0 (`self.UpMovingTime`)))
        (goto _label)
        (else
          (`TimelineComponent.SetPlayRate` (`self.MoveDoor`) (/ 1.0 (`self.UpMovingTime`)))
          (goto _label))))))

(event `self.ReceiveBeginPlay`
  (bind _movedoor (`self.MoveDoor`))
  (if (`self.Open`)
    (`TimelineComponent.SetPlaybackPosition` _movedoor (`TimelineComponent.GetTimelineLength` _movedoor) false true)))

(fn `UserConstructionScript`)