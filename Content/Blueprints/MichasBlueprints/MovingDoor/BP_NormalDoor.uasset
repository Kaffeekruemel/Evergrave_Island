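; BP_NormalDoor is a hinged door Blueprint that swings open and closed through its OpenDoor and CloseDoor events.
; A timeline, played or reversed, scales Angle to set the SMDoor mesh's relative rotation on one axis, chosen by flags prioritized Z, Y, then X.
; BeginPlay derives the play rate from OpeningLength and, if Open is set, moves the timeline to its end without firing update events.
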(event `self.ReceiveBeginPlay`
  (bind _timeline_0 (`self.Timeline_0`))
  (`TimelineComponent.SetPlayRate` (`self.Timeline_0`) (/ 1.0 (`self.OpeningLength`)))
  (if (`self.Open`)
    (`TimelineComponent.SetPlaybackPosition` _timeline_0 (`TimelineComponent.GetTimelineLength` _timeline_0) false true)))

(event `OpenDoor`
  (bind _sm_door (`self.SM_Door`))
  (set `self.Open` true)
  (bind (_direction _newtrack_0) (`Timeline|Timeline_0` :!label _label)
    (:`Update`
      (if (`self.Z`)
        (bind _returnvalue (* _newtrack_0 (`self.Angle`)))
        (`SceneComponent.K2_SetRelativeRotation` _sm_door (`KismetMathLibrary.MakeRotator` 0.0 0.0 _returnvalue) false false)
        (elif (`self.Y`)
          (`SceneComponent.K2_SetRelativeRotation` _sm_door (`KismetMathLibrary.MakeRotator` 0.0 _returnvalue) false false)
          (elif (`self.X`)
            (`SceneComponent.K2_SetRelativeRotation` _sm_door (`KismetMathLibrary.MakeRotator` _returnvalue) false false)))))))

(event `CloseDoor`
  (set `self.Open` false)
  (goto _label :!via `Reverse`))

(fn `UserConstructionScript`)