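; Multi-lever door puzzle controller that triggers a door once all assigned BP_MOTUDoorLever levers (two to five) are pressed.
; Tick polls the levers through nested branches, one per lever count, until AlreadyUsed latches it to a single use.
; It starts the first move of an UpAndDownDoor if set, otherwise opens or closes a NormalDoor based on its timeline position.
; BeginPlay prints warnings when either required lever is missing.
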(event `self.ReceiveBeginPlay`
  (`|ExecutionSequence`
    (:`then_0`
      (if (not (`KismetSystemLibrary.IsValid` (`self.Lever1`)))
        (`KismetSystemLibrary.PrintString` "ButtonOneIsMissing"))
      (if (not (`KismetSystemLibrary.IsValid` (`self.Lever2`)))
        (`KismetSystemLibrary.PrintString` "ButtonTwoIsMissing"))
      (if (`KismetSystemLibrary.IsValid` (`self.Lever3`))
        (if (`KismetSystemLibrary.IsValid` (`self.Lever4`))
          (if (`KismetSystemLibrary.IsValid` (`self.Lever5`))
            _))))))

(event `self.ReceiveTick`
  (params (DeltaSeconds :type "Float (single-precision)"))
  (bind _normaldoor (`self.NormalDoor`))
  (bind _normaldoor_2 (`self.NormalDoor`))
  (bind _normaldoor_3 (`self.NormalDoor`))
  (bind _normaldoor_4 (`self.NormalDoor`))
  (if (`self.AlreadyUsed`)
    _
    (elif (or (`KismetSystemLibrary.IsValid` (`self.NormalDoor`)) (`KismetSystemLibrary.IsValid` (`self.UpAndDownDoor`)))
      (if (and (`KismetSystemLibrary.IsValid` (`self.Lever1`)) (`KismetSystemLibrary.IsValid` (`self.Lever2`)))
        (bind _asbp_motudoor_lever (cast `/Game/Blueprints/MichasBlueprints/Levers/DoorLever/MultipleLevers/BP_MOTUDoorLever` (`self.Lever1`)))
        (bind _asbp_motudoor_lever_2 (cast `/Game/Blueprints/MichasBlueprints/Levers/DoorLever/MultipleLevers/BP_MOTUDoorLever` (`self.Lever2`)))
        (if (and (not (`KismetSystemLibrary.IsValid` (`self.Lever3`))) (not (`KismetSystemLibrary.IsValid` (`self.Lever4`))) (not (`KismetSystemLibrary.IsValid` (`self.Lever5`))))
          (bind _pressed (`/Game/Blueprints/MichasBlueprints/Levers/DoorLever/MultipleLevers/BP_MOTUDoorLever.Pressed` _asbp_motudoor_lever))
          (bind _pressed_2 (`/Game/Blueprints/MichasBlueprints/Levers/DoorLever/MultipleLevers/BP_MOTUDoorLever.Pressed` _asbp_motudoor_lever_2))
          (bind _returnvalue (and _pressed _pressed_2))
          (if _returnvalue
            (if (`KismetSystemLibrary.IsValid` (`self.UpAndDownDoor`))
              (bind _asbp_comlexe_door (cast `/Game/Blueprints/MichasBlueprints/MovingDoor/BP_ComlexeDoor` (`self.UpAndDownDoor`)))
              (`/Game/Blueprints/MichasBlueprints/MovingDoor/BP_ComlexeDoor.StartFirstMove` _asbp_comlexe_door _returnvalue)
              (set `self.AlreadyUsed` true)
              (elif (`KismetSystemLibrary.IsValid` (`self.NormalDoor`))
                (bind _asbp_normal_door (cast `/Game/Blueprints/MichasBlueprints/MovingDoor/BP_NormalDoor` (`self.NormalDoor`)))
                (if (> (`TimelineComponent.GetPlaybackPosition` (`/Game/Blueprints/MichasBlueprints/MovingDoor/BP_NormalDoor.Timeline_0` _asbp_normal_door)) 1.0)
                  (bind _asbp_normal_door_2 (cast `/Game/Blueprints/MichasBlueprints/MovingDoor/BP_NormalDoor` _normaldoor_2))
                  (`/Game/Blueprints/MichasBlueprints/MovingDoor/BP_NormalDoor.CloseDoor` _asbp_normal_door_2)
                  (set `self.AlreadyUsed` true)
                  (else
                    (bind _asbp_normal_door_3 (cast `/Game/Blueprints/MichasBlueprints/MovingDoor/BP_NormalDoor` _normaldoor_2))
                    (`/Game/Blueprints/MichasBlueprints/MovingDoor/BP_NormalDoor.OpenDoor` _asbp_normal_door_3)
                    (set `self.AlreadyUsed` true)))
                (else
                  (`KismetSystemLibrary.PrintString` "No Doors Selected")))))
          (else
            (bind _asbp_motudoor_lever_3 (cast `/Game/Blueprints/MichasBlueprints/Levers/DoorLever/MultipleLevers/BP_MOTUDoorLever` (`self.Lever3`)))
            (if (and (not (`KismetSystemLibrary.IsValid` (`self.Lever4`))) (not (`KismetSystemLibrary.IsValid` (`self.Lever5`))))
              (bind _pressed_3 (`/Game/Blueprints/MichasBlueprints/Levers/DoorLever/MultipleLevers/BP_MOTUDoorLever.Pressed` _asbp_motudoor_lever_3))
              (bind _returnvalue_2 (and _pressed _pressed_2 _pressed_3))
              (if _returnvalue_2
                (if (`KismetSystemLibrary.IsValid` (`self.UpAndDownDoor`))
                  (bind _asbp_comlexe_door_2 (cast `/Game/Blueprints/MichasBlueprints/MovingDoor/BP_ComlexeDoor` (`self.UpAndDownDoor`)))
                  (`/Game/Blueprints/MichasBlueprints/MovingDoor/BP_ComlexeDoor.StartFirstMove` _asbp_comlexe_door_2 _returnvalue_2)
                  (set `self.AlreadyUsed` true)
                  (elif (`KismetSystemLibrary.IsValid` (`self.NormalDoor`))
                    (bind _asbp_normal_door_4 (cast `/Game/Blueprints/MichasBlueprints/MovingDoor/BP_NormalDoor` (`self.NormalDoor`)))
                    (if (> (`TimelineComponent.GetPlaybackPosition` (`/Game/Blueprints/MichasBlueprints/MovingDoor/BP_NormalDoor.Timeline_0` _asbp_normal_door_4)) 1.0)
                      (bind _asbp_normal_door_5 (cast `/Game/Blueprints/MichasBlueprints/MovingDoor/BP_NormalDoor` _normaldoor_3))
                      (`/Game/Blueprints/MichasBlueprints/MovingDoor/BP_NormalDoor.CloseDoor` _asbp_normal_door_5)
                      (set `self.AlreadyUsed` true)
                      (else
                        (bind _asbp_normal_door_6 (cast `/Game/Blueprints/MichasBlueprints/MovingDoor/BP_NormalDoor` _normaldoor_3))
                        (`/Game/Blueprints/MichasBlueprints/MovingDoor/BP_NormalDoor.OpenDoor` _asbp_normal_door_6)
                        (set `self.AlreadyUsed` true)))
                    (else
                      (`KismetSystemLibrary.PrintString` "No Doors Selected")))))
              (else
                (bind _asbp_motudoor_lever_4 (cast `/Game/Blueprints/MichasBlueprints/Levers/DoorLever/MultipleLevers/BP_MOTUDoorLever` (`self.Lever4`)))
                (if (not (`KismetSystemLibrary.IsValid` (`self.Lever5`)))
                  (bind _pressed_4 (`/Game/Blueprints/MichasBlueprints/Levers/DoorLever/MultipleLevers/BP_MOTUDoorLever.Pressed` _asbp_motudoor_lever_4))
                  (bind _returnvalue_3 (and _pressed _pressed_2 _pressed_3 _pressed_4))
                  (if _returnvalue_3
                    (if (`KismetSystemLibrary.IsValid` (`self.UpAndDownDoor`))
                      (bind _asbp_comlexe_door_3 (cast `/Game/Blueprints/MichasBlueprints/MovingDoor/BP_ComlexeDoor` (`self.UpAndDownDoor`)))
                      (`/Game/Blueprints/MichasBlueprints/MovingDoor/BP_ComlexeDoor.StartFirstMove` _asbp_comlexe_door_3 _returnvalue_3)
                      (set `self.AlreadyUsed` true)
                      (elif (`KismetSystemLibrary.IsValid` (`self.NormalDoor`))
                        (bind _asbp_normal_door_7 (cast `/Game/Blueprints/MichasBlueprints/MovingDoor/BP_NormalDoor` (`self.NormalDoor`)))
                        (if (> (`TimelineComponent.GetPlaybackPosition` (`/Game/Blueprints/MichasBlueprints/MovingDoor/BP_NormalDoor.Timeline_0` _asbp_normal_door_7)) 1.0)
                          (bind _asbp_normal_door_8 (cast `/Game/Blueprints/MichasBlueprints/MovingDoor/BP_NormalDoor` _normaldoor_4))
                          (`/Game/Blueprints/MichasBlueprints/MovingDoor/BP_NormalDoor.CloseDoor` _asbp_normal_door_8)
                          (set `self.AlreadyUsed` true)
                          (else
                            (bind _asbp_normal_door_9 (cast `/Game/Blueprints/MichasBlueprints/MovingDoor/BP_NormalDoor` _normaldoor_4))
                            (`/Game/Blueprints/MichasBlueprints/MovingDoor/BP_NormalDoor.OpenDoor` _asbp_normal_door_9)
                            (set `self.AlreadyUsed` true)))
                        (else
                          (`KismetSystemLibrary.PrintString` "No Doors Selected")))))
                  (else
                    (bind _asbp_motudoor_lever_5 (cast `/Game/Blueprints/MichasBlueprints/Levers/DoorLever/MultipleLevers/BP_MOTUDoorLever` (`self.Lever5`)))
                    (bind _returnvalue_4 (and _pressed _pressed_2 _pressed_3 _pressed_4 (`/Game/Blueprints/MichasBlueprints/Levers/DoorLever/MultipleLevers/BP_MOTUDoorLever.Pressed` _asbp_motudoor_lever_5)))
                    (if _returnvalue_4
                      (if (`KismetSystemLibrary.IsValid` (`self.UpAndDownDoor`))
                        (bind _asbp_comlexe_door_4 (cast `/Game/Blueprints/MichasBlueprints/MovingDoor/BP_ComlexeDoor` (`self.UpAndDownDoor`)))
                        (`/Game/Blueprints/MichasBlueprints/MovingDoor/BP_ComlexeDoor.StartFirstMove` _asbp_comlexe_door_4 _returnvalue_4)
                        (set `self.AlreadyUsed` true)
                        (elif (`KismetSystemLibrary.IsValid` (`self.NormalDoor`))
                          (bind _asbp_normal_door_10 (cast `/Game/Blueprints/MichasBlueprints/MovingDoor/BP_NormalDoor` (`self.NormalDoor`)))
                          (if (> (`TimelineComponent.GetPlaybackPosition` (`/Game/Blueprints/MichasBlueprints/MovingDoor/BP_NormalDoor.Timeline_0` _asbp_normal_door_10)) 1.0)
                            (bind _asbp_normal_door_11 (cast `/Game/Blueprints/MichasBlueprints/MovingDoor/BP_NormalDoor` _normaldoor))
                            (`/Game/Blueprints/MichasBlueprints/MovingDoor/BP_NormalDoor.CloseDoor` _asbp_normal_door_11)
                            (set `self.AlreadyUsed` true)
                            (else
                              (bind _asbp_normal_door_12 (cast `/Game/Blueprints/MichasBlueprints/MovingDoor/BP_NormalDoor` _normaldoor))
                              (`/Game/Blueprints/MichasBlueprints/MovingDoor/BP_NormalDoor.OpenDoor` _asbp_normal_door_12)
                              (set `self.AlreadyUsed` true)))
                          (else
                            (`KismetSystemLibrary.PrintString` "No Doors Selected")))))))))))))))

(fn `UserConstructionScript`)