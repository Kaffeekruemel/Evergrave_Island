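; Multi-lever puzzle controller that blows up a linked Destructable actor once all its assigned levers are pressed.
; Supports two to five BP_MultipleOTUExplosionLever references in Button1–5, filled in order; BeginPlay prints a warning if either of the first two is missing.
; Tick polls each lever's Pressed flag through nested validity checks and casts, then spawns an explosion emitter at the target's location and scale and destroys it.
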(event `self.ReceiveBeginPlay`
  (`|ExecutionSequence`
    (:`then_0`
      (if (not (`KismetSystemLibrary.IsValid` (`self.Button1`)))
        (`KismetSystemLibrary.PrintString` "ButtonOneIsMissing"))
      (if (not (`KismetSystemLibrary.IsValid` (`self.Button2`)))
        (`KismetSystemLibrary.PrintString` "ButtonTwoIsMissing"))
      (if (`KismetSystemLibrary.IsValid` (`self.Button3`))
        (if (`KismetSystemLibrary.IsValid` (`self.Button4`))
          (if (`KismetSystemLibrary.IsValid` (`self.Button5`))
            _))))))

(event `self.ReceiveTick`
  (params (DeltaSeconds :type "Float (single-precision)"))
  (bind _destructable (`self.Destructable`))
  (bind _destructable_2 (`self.Destructable`))
  (bind _destructable_3 (`self.Destructable`))
  (bind _destructable_4 (`self.Destructable`))
  (if (`KismetSystemLibrary.IsValid` (`self.Destructable`))
    (if (and (`KismetSystemLibrary.IsValid` (`self.Button1`)) (`KismetSystemLibrary.IsValid` (`self.Button2`)))
      (bind _asbp_multiple_otuexplosion_lever (cast `/Game/Blueprints/MichasBlueprints/Levers/DestructionLever/MultipleLever/BP_MultipleOTUExplosionLever` (`self.Button1`)))
      (bind _asbp_multiple_otuexplosion_lever_2 (cast `/Game/Blueprints/MichasBlueprints/Levers/DestructionLever/MultipleLever/BP_MultipleOTUExplosionLever` (`self.Button2`)))
      (if (and (not (`KismetSystemLibrary.IsValid` (`self.Button3`))) (not (`KismetSystemLibrary.IsValid` (`self.Button4`))) (not (`KismetSystemLibrary.IsValid` (`self.Button5`))))
        (bind _pressed (`/Game/Blueprints/MichasBlueprints/Levers/DestructionLever/MultipleLever/BP_MultipleOTUExplosionLever.Pressed` _asbp_multiple_otuexplosion_lever))
        (bind _pressed_2 (`/Game/Blueprints/MichasBlueprints/Levers/DestructionLever/MultipleLever/BP_MultipleOTUExplosionLever.Pressed` _asbp_multiple_otuexplosion_lever_2))
        (if (and _pressed _pressed_2)
          (`GameplayStatics.SpawnEmitterAtLocation` "/Game/Base/StarterContent/Particles/P_Explosion.P_Explosion" (`self.K2_GetActorLocation` _destructable_2) (struct) (`self.GetActorScale3D` _destructable_2))
          (`self.K2_DestroyActor` (`self.Destructable`)))
        (else
          (bind _asbp_multiple_otuexplosion_lever_3 (cast `/Game/Blueprints/MichasBlueprints/Levers/DestructionLever/MultipleLever/BP_MultipleOTUExplosionLever` (`self.Button3`)))
          (if (and (not (`KismetSystemLibrary.IsValid` (`self.Button4`))) (not (`KismetSystemLibrary.IsValid` (`self.Button5`))))
            (bind _pressed_3 (`/Game/Blueprints/MichasBlueprints/Levers/DestructionLever/MultipleLever/BP_MultipleOTUExplosionLever.Pressed` _asbp_multiple_otuexplosion_lever_3))
            (if (and _pressed _pressed_2 _pressed_3)
              (`GameplayStatics.SpawnEmitterAtLocation` "/Game/Base/StarterContent/Particles/P_Explosion.P_Explosion" (`self.K2_GetActorLocation` _destructable_3) (struct) (`self.GetActorScale3D` _destructable_3))
              (`self.K2_DestroyActor` (`self.Destructable`)))
            (else
              (bind _asbp_multiple_otuexplosion_lever_4 (cast `/Game/Blueprints/MichasBlueprints/Levers/DestructionLever/MultipleLever/BP_MultipleOTUExplosionLever` (`self.Button4`)))
              (if (not (`KismetSystemLibrary.IsValid` (`self.Button5`)))
                (bind _pressed_4 (`/Game/Blueprints/MichasBlueprints/Levers/DestructionLever/MultipleLever/BP_MultipleOTUExplosionLever.Pressed` _asbp_multiple_otuexplosion_lever_4))
                (if (and _pressed _pressed_2 _pressed_3 _pressed_4)
                  (`GameplayStatics.SpawnEmitterAtLocation` "/Game/Base/StarterContent/Particles/P_Explosion.P_Explosion" (`self.K2_GetActorLocation` _destructable_4) (struct) (`self.GetActorScale3D` _destructable_4))
                  (`self.K2_DestroyActor` (`self.Destructable`)))
                (else
                  (bind _asbp_multiple_otuexplosion_lever_5 (cast `/Game/Blueprints/MichasBlueprints/Levers/DestructionLever/MultipleLever/BP_MultipleOTUExplosionLever` (`self.Button5`)))
                  (if (and _pressed _pressed_2 _pressed_3 _pressed_4 (`/Game/Blueprints/MichasBlueprints/Levers/DestructionLever/MultipleLever/BP_MultipleOTUExplosionLever.Pressed` _asbp_multiple_otuexplosion_lever_5))
                    (`GameplayStatics.SpawnEmitterAtLocation` "/Game/Base/StarterContent/Particles/P_Explosion.P_Explosion" (`self.K2_GetActorLocation` _destructable) (struct) (`self.GetActorScale3D` _destructable))
                    (`self.K2_DestroyActor` (`self.Destructable`))))))))))))

(fn `UserConstructionScript`)