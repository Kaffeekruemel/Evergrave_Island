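; Puzzle controller that enables a BP_Moving_Platform once all of its assigned levers are pressed.
; On BeginPlay it prints a warning if either of the two required levers is missing; three more are optional.
; Each Tick it polls Pressed on the BP_MultipleOTUMovingLever references through nested checks that expect slots filled in order.
; When all are pressed it sets the platform's CanMove to true, and never clears it.
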(event `self.ReceiveBeginPlay`
  (`|ExecutionSequence`
    (:`then_0`
      (if (not (`KismetSystemLibrary.IsValid` (`self.Lever1`)))
        (`KismetSystemLibrary.PrintString` "ButtonOneIsMissing"))
      (if (not (`KismetSystemLibrary.IsValid` (`self.Lever2`)))
        (`KismetSystemLibrary.PrintString` "ButtonTwoIsMissing"))
      (if (`KismetSystemLibrary.IsValid` (`self.Lever3`))
        (if (`KismetSystemLibrary.IsValid` (`self.Lever4`))
          (if (`KismetSystemLibrary.IsValid` (`self.Lever5`))
            _))))))

(event `self.ReceiveTick`
  (params (DeltaSeconds :type "Float (single-precision)"))
  (if (`KismetSystemLibrary.IsValid` (`self.MovingPlatform`))
    (if (and (`KismetSystemLibrary.IsValid` (`self.Lever1`)) (`KismetSystemLibrary.IsValid` (`self.Lever2`)))
      (bind _asbp_multiple_otumoving_lever (cast `/Game/Blueprints/MichasBlueprints/Levers/MovingLever/MultipleLever/BP_MultipleOTUMovingLever` (`self.Lever1`)))
      (bind _asbp_multiple_otumoving_lever_2 (cast `/Game/Blueprints/MichasBlueprints/Levers/MovingLever/MultipleLever/BP_MultipleOTUMovingLever` (`self.Lever2`)))
      (if (and (not (`KismetSystemLibrary.IsValid` (`self.Lever3`))) (not (`KismetSystemLibrary.IsValid` (`self.Lever4`))) (not (`KismetSystemLibrary.IsValid` (`self.Lever5`))))
        (bind _pressed (`/Game/Blueprints/MichasBlueprints/Levers/MovingLever/MultipleLever/BP_MultipleOTUMovingLever.Pressed` _asbp_multiple_otumoving_lever))
        (bind _pressed_2 (`/Game/Blueprints/MichasBlueprints/Levers/MovingLever/MultipleLever/BP_MultipleOTUMovingLever.Pressed` _asbp_multiple_otumoving_lever_2))
        (if (and _pressed _pressed_2)
          (bind _asbp_moving_platform (cast `/Game/Blueprints/MichasBlueprints/MovingPlatform/BP_Moving_Platform` (`self.MovingPlatform`)))
          (set `/Game/Blueprints/MichasBlueprints/MovingPlatform/BP_Moving_Platform.CanMove` true _asbp_moving_platform))
        (else
          (bind _asbp_multiple_otumoving_lever_3 (cast `/Game/Blueprints/MichasBlueprints/Levers/MovingLever/MultipleLever/BP_MultipleOTUMovingLever` (`self.Lever3`)))
          (if (and (not (`KismetSystemLibrary.IsValid` (`self.Lever4`))) (not (`KismetSystemLibrary.IsValid` (`self.Lever5`))))
            (bind _pressed_3 (`/Game/Blueprints/MichasBlueprints/Levers/MovingLever/MultipleLever/BP_MultipleOTUMovingLever.Pressed` _asbp_multiple_otumoving_lever_3))
            (if (and _pressed _pressed_2 _pressed_3)
              (bind _asbp_moving_platform_2 (cast `/Game/Blueprints/MichasBlueprints/MovingPlatform/BP_Moving_Platform` (`self.MovingPlatform`)))
              (set `/Game/Blueprints/MichasBlueprints/MovingPlatform/BP_Moving_Platform.CanMove` true _asbp_moving_platform_2))
            (else
              (bind _asbp_multiple_otumoving_lever_4 (cast `/Game/Blueprints/MichasBlueprints/Levers/MovingLever/MultipleLever/BP_MultipleOTUMovingLever` (`self.Lever4`)))
              (if (not (`KismetSystemLibrary.IsValid` (`self.Lever5`)))
                (bind _pressed_4 (`/Game/Blueprints/MichasBlueprints/Levers/MovingLever/MultipleLever/BP_MultipleOTUMovingLever.Pressed` _asbp_multiple_otumoving_lever_4))
                (if (and _pressed _pressed_2 _pressed_3 _pressed_4)
                  (bind _asbp_moving_platform_3 (cast `/Game/Blueprints/MichasBlueprints/MovingPlatform/BP_Moving_Platform` (`self.MovingPlatform`)))
                  (set `/Game/Blueprints/MichasBlueprints/MovingPlatform/BP_Moving_Platform.CanMove` true _asbp_moving_platform_3))
                (else
                  (bind _asbp_multiple_otumoving_lever_5 (cast `/Game/Blueprints/MichasBlueprints/Levers/MovingLever/MultipleLever/BP_MultipleOTUMovingLever` (`self.Lever5`)))
                  (if (and _pressed _pressed_2 _pressed_3 _pressed_4 (`/Game/Blueprints/MichasBlueprints/Levers/MovingLever/MultipleLever/BP_MultipleOTUMovingLever.Pressed` _asbp_multiple_otumoving_lever_5))
                    (bind _asbp_moving_platform_4 (cast `/Game/Blueprints/MichasBlueprints/MovingPlatform/BP_Moving_Platform` (`self.MovingPlatform`)))
                    (set `/Game/Blueprints/MichasBlueprints/MovingPlatform/BP_Moving_Platform.CanMove` true _asbp_moving_platform_4)))))))))))

(fn `UserConstructionScript`)