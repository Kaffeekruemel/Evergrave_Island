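; Puzzle controller that powers an updraft once all of its linked levers are pressed.
; Takes two required and up to three optional lever references, printing a warning on BeginPlay if either required one is missing.
; Tick polls each assigned lever's Pressed flag through nested validity checks, then sets the Updraft_BP's lift speed when all are pressed.
; Nothing here resets the speed when a lever is released.
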(event `self.ReceiveBeginPlay`
  (`|ExecutionSequence`
    (:`then_0`
      (if (not (`KismetSystemLibrary.IsValid` (`self.Button1`)))
        (`KismetSystemLibrary.PrintString` "ButtonOneIsMissing"))
      (if (not (`KismetSystemLibrary.IsValid` (`self.Button2`)))
        (`KismetSystemLibrary.PrintString` "ButtonTwoIsMissing"))
      (if (`KismetSystemLibrary.IsValid` (`self.Button3`))
        (if (`KismetSystemLibrary.IsValid` (`self.Button4`))
          (if (`KismetSystemLibrary.IsValid` (`self.Button5`))
            _))))))

(event `self.ReceiveTick`
  (params (DeltaSeconds :type "Float (single-precision)"))
  (if (`KismetSystemLibrary.IsValid` (`self.Updraft`))
    (if (and (`KismetSystemLibrary.IsValid` (`self.Button1`)) (`KismetSystemLibrary.IsValid` (`self.Button2`)))
      (bind _asbp_motulever (cast `/Game/Blueprints/MichasBlueprints/Levers/UpdraftLever/MultipleLever/BP_MOTULever` (`self.Button1`)))
      (bind _asbp_motulever_2 (cast `/Game/Blueprints/MichasBlueprints/Levers/UpdraftLever/MultipleLever/BP_MOTULever` (`self.Button2`)))
      (if (and (not (`KismetSystemLibrary.IsValid` (`self.Button3`))) (not (`KismetSystemLibrary.IsValid` (`self.Button4`))) (not (`KismetSystemLibrary.IsValid` (`self.Button5`))))
        (bind _pressed (`/Game/Blueprints/MichasBlueprints/Levers/UpdraftLever/MultipleLever/BP_MOTULever.Pressed` _asbp_motulever))
        (bind _pressed_2 (`/Game/Blueprints/MichasBlueprints/Levers/UpdraftLever/MultipleLever/BP_MOTULever.Pressed` _asbp_motulever_2))
        (if (and _pressed _pressed_2)
          (bind _asupdraft_bp (cast `/Game/Base/DynamicParaglider/Blueprints/Updraft/Updraft_BP` (`self.Updraft`)))
          (`/Game/Base/DynamicParaglider/Blueprints/Updraft/Updraft_BP.SetLiftspeed` _asupdraft_bp (`self.LiftSpeed`)))
        (else
          (bind _asbp_motulever_3 (cast `/Game/Blueprints/MichasBlueprints/Levers/UpdraftLever/MultipleLever/BP_MOTULever` (`self.Button3`)))
          (if (and (not (`KismetSystemLibrary.IsValid` (`self.Button4`))) (not (`KismetSystemLibrary.IsValid` (`self.Button5`))))
            (bind _pressed_3 (`/Game/Blueprints/MichasBlueprints/Levers/UpdraftLever/MultipleLever/BP_MOTULever.Pressed` _asbp_motulever_3))
            (if (and _pressed _pressed_2 _pressed_3)
              (bind _asupdraft_bp_2 (cast `/Game/Base/DynamicParaglider/Blueprints/Updraft/Updraft_BP` (`self.Updraft`)))
              (`/Game/Base/DynamicParaglider/Blueprints/Updraft/Updraft_BP.SetLiftspeed` _asupdraft_bp_2 (`self.LiftSpeed`)))
            (else
              (bind _asbp_motulever_4 (cast `/Game/Blueprints/MichasBlueprints/Levers/UpdraftLever/MultipleLever/BP_MOTULever` (`self.Button4`)))
              (if (not (`KismetSystemLibrary.IsValid` (`self.Button5`)))
                (bind _pressed_4 (`/Game/Blueprints/MichasBlueprints/Levers/UpdraftLever/MultipleLever/BP_MOTULever.Pressed` _asbp_motulever_4))
                (if (and _pressed _pressed_2 _pressed_3 _pressed_4)
                  (bind _asupdraft_bp_3 (cast `/Game/Base/DynamicParaglider/Blueprints/Updraft/Updraft_BP` (`self.Updraft`)))
                  (`/Game/Base/DynamicParaglider/Blueprints/Updraft/Updraft_BP.SetLiftspeed` _asupdraft_bp_3 (`self.LiftSpeed`)))
                (else
                  (bind _asbp_motulever_5 (cast `/Game/Blueprints/MichasBlueprints/Levers/UpdraftLever/MultipleLever/BP_MOTULever` (`self.Button5`)))
                  (if (and _pressed _pressed_2 _pressed_3 _pressed_4 (`/Game/Blueprints/MichasBlueprints/Levers/UpdraftLever/MultipleLever/BP_MOTULever.Pressed` _asbp_motulever_5))
                    (bind _asupdraft_bp_4 (cast `/Game/Base/DynamicParaglider/Blueprints/Updraft/Updraft_BP` (`self.Updraft`)))
                    (`/Game/Base/DynamicParaglider/Blueprints/Updraft/Updraft_BP.SetLiftspeed` _asupdraft_bp_4 (`self.LiftSpeed`))))))))))))

(fn `UserConstructionScript`)