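; Checkpoint indicator actor that shows an active or inactive state by moving Cube1 vertically and recoloring Cube.
; The UpAndDown event takes an Active flag: when true, the Movemnt timeline applies the green material, then hands over to Timeline_0.
; When false, it stops Timeline_0 and runs Timeline_1 with the pink material.
; All three timelines drive Cube1's relative Z, scaled by Movment1.
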(event `self.ReceiveActorBeginOverlap`
  (params (OtherActor :type "Actor Object Reference")))

(event `UpAndDown`
  (params (Active :type Boolean))
  (if Active
    (bind (_direction _newtrack_0) (`Timeline|Movemnt` :!via `PlayFromStart`)
      (:`Update`
        (`SceneComponent.K2_SetRelativeLocation` (`self.Cube1`) (`KismetMathLibrary.MakeVector` 0.0 0.0 (* _newtrack_0 (`self.Movment1`))) false false)
        (`PrimitiveComponent.SetMaterial` (`self.cube`) 0 "/Game/M_Cape_Green.M_Cape_Green"))
      (:`Finished`
        (bind (_direction_2 _newtrack_0_2) (`Timeline|Timeline_0` :!label _label)
          (:`Update`
            (`SceneComponent.K2_SetRelativeLocation` (`self.Cube1`) (`KismetMathLibrary.MakeVector` 0.0 0.0 (* _newtrack_0_2 (`self.Movment1`))) false false)))))
    (else
      (`|ExecutionSequence`
        (:`then_0`
          (goto _label :!via `Stop`))
        (:`then_1`
          (bind (_direction_3 _newtrack_0_3) (`Timeline|Timeline_1` :!via `PlayFromStart`)
            (:`Update`
              (`SceneComponent.K2_SetRelativeLocation` (`self.Cube1`) (`KismetMathLibrary.MakeVector` 0.0 0.0 (* _newtrack_0_3 (`self.Movment1`))) false false)
              (`PrimitiveComponent.SetMaterial` (`self.cube`) 0 "/Game/Enviroment/Props/Meshes/Lever/PinkLever.PinkLever"))))))))

(fn `UserConstructionScript`)