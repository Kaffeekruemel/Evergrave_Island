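; Pressure button that drives one linked door, either a BP_ComlexeDoor or a BP_NormalDoor, with the complex door taking priority.
; Box overlap checks the button's height before triggering the door, then plays a timeline that moves the button by ButtonMovement.
; Ending overlap reverses the timeline and signals the door back, unless OneTimeUse is set.
; Older MoveComponentTo and clamping logic remains disconnected.
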(event `self.ReceiveTick`
  (params (DeltaSeconds :type "Float (single-precision)")))

(event `self.Box.OnComponentBeginOverlap`
  (params (OverlappedComponent :type "PrimitiveComponent Object Reference") (OtherActor :type "Actor Object Reference") (OtherComp :type "PrimitiveComponent Object Reference") (OtherBodyIndex :type Integer) (bFromSweep :type Boolean) (SweepResult :type "HitResult Structure (by ref)"))
  (bind (_relativelocation_x _relativelocation_y _relativelocation_z) (`KismetMathLibrary.BreakVector` (`SceneComponent.RelativeLocation` (`self.button`))))
  (`|ExecutionSequence`
    (:`then_0`
      (if (>= _relativelocation_z (`self.ButtonMovement`))
        (bind _output_get (set `self.ButtonPressed` true))
        (if (`KismetSystemLibrary.IsValid` (`self.UpAndDownDoor`))
          (bind _asbp_comlexe_door (cast `/Game/Blueprints/MichasBlueprints/MovingDoor/BP_ComlexeDoor` (`self.UpAndDownDoor`)))
          (`/Game/Blueprints/MichasBlueprints/MovingDoor/BP_ComlexeDoor.StartFirstMove` _asbp_comlexe_door _output_get)
          (elif (`KismetSystemLibrary.IsValid` (`self.NormalDoor`))
            (bind _asbp_normal_door (cast `/Game/Blueprints/MichasBlueprints/MovingDoor/BP_NormalDoor` (`self.NormalDoor`)))
            (`/Game/Blueprints/MichasBlueprints/MovingDoor/BP_NormalDoor.OpenDoor` _asbp_normal_door)
            (else
              (`KismetSystemLibrary.PrintString` "No Doors Selected"))))))
    (:`then_1`
      (bind (_direction _newtrack_0) (`Timeline|Timeline_0` :!label _label)
        (:`Update`
          (`SceneComponent.K2_SetRelativeLocation` (`self.button`) (`KismetMathLibrary.MakeVector` 0.0 0.0 (* _newtrack_0 (`self.ButtonMovement`))) false false))))))

(event `self.Box.OnComponentEndOverlap`
  (params (OverlappedComponent :type "PrimitiveComponent Object Reference") (OtherActor :type "Actor Object Reference") (OtherComp :type "PrimitiveComponent Object Reference") (OtherBodyIndex :type Integer))
  (if (not (`self.OneTimeUse`))
    (`|ExecutionSequence`
      (:`then_0`
        (goto _label :!via `Reverse`))
      (:`then_1`
        (bind _output_get (set `self.ButtonPressed` false))
        (if (`KismetSystemLibrary.IsValid` (`self.UpAndDownDoor`))
          (bind _asbp_comlexe_door (cast `/Game/Blueprints/MichasBlueprints/MovingDoor/BP_ComlexeDoor` (`self.UpAndDownDoor`)))
          (`/Game/Blueprints/MichasBlueprints/MovingDoor/BP_ComlexeDoor.StartFirstMove` _asbp_comlexe_door _output_get)
          (elif (`KismetSystemLibrary.IsValid` (`self.NormalDoor`))
            (bind _asbp_normal_door (cast `/Game/Blueprints/MichasBlueprints/MovingDoor/BP_NormalDoor` (`self.NormalDoor`)))
            (`/Game/Blueprints/MichasBlueprints/MovingDoor/BP_NormalDoor.CloseDoor` _asbp_normal_door)
            (else
              (`KismetSystemLibrary.PrintString` "No Doors Selected"))))))))

(fn `UserConstructionScript`)