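; One-time floor button that operates a linked door when something overlaps its box.
; An overlap eases the button down unless it is already at or below a height threshold, and nothing here raises it again.
; If it ends low enough, it starts the first move of the up-and-down door or, without one, toggles the normal door open or closed.
; It prints a message when neither door is assigned.
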(event `self.Box.OnComponentBeginOverlap`
  (params (OverlappedComponent :type "PrimitiveComponent Object Reference") (OtherActor :type "Actor Object Reference") (OtherComp :type "PrimitiveComponent Object Reference") (OtherBodyIndex :type Integer) (bFromSweep :type Boolean) (SweepResult :type "HitResult Structure (by ref)"))
  (bind _normal_door (`self.Normal Door`))
  (bind _button (`self.button`))
  (bind (_relativelocation_x _relativelocation_y _relativelocation_z) (`KismetMathLibrary.BreakVector` (`SceneComponent.RelativeLocation` (`self.button`))))
  (bind (_relativelocation_x_2 _relativelocation_y_2 _relativelocation_z_2) (`KismetMathLibrary.BreakVector` (`SceneComponent.RelativeLocation` (`self.button`))))
  (bind (_relativelocation_x_3 _relativelocation_y_3 _relativelocation_z_3) (`KismetMathLibrary.BreakVector` (`SceneComponent.RelativeLocation` _button)))
  (if (not (>= 10.0 _relativelocation_z))
    (`KismetSystemLibrary.MoveComponentTo` _button (`KismetMathLibrary.MakeVector` _relativelocation_x_3 _relativelocation_y_3 (- _relativelocation_z_3 (`self.ButtonMovement`))) (struct) true false 0.3)
    (if (<= _relativelocation_z_2 10.0)
      (bind _output_get (set `self.ButtonPressed` true))
      (if (`KismetSystemLibrary.IsValid` (`self.UpAndDownDoor`))
        (bind _asbp_comlexe_door (cast `/Game/Blueprints/MichasBlueprints/MovingDoor/BP_ComlexeDoor` (`self.UpAndDownDoor`)))
        (`/Game/Blueprints/MichasBlueprints/MovingDoor/BP_ComlexeDoor.StartFirstMove` _asbp_comlexe_door _output_get)
        (elif (`KismetSystemLibrary.IsValid` (`self.Normal Door`))
          (bind _asbp_normal_door (cast `/Game/Blueprints/MichasBlueprints/MovingDoor/BP_NormalDoor` _normal_door))
          (if (`/Game/Blueprints/MichasBlueprints/MovingDoor/BP_NormalDoor.Open` _asbp_normal_door)
            (bind _asbp_normal_door_2 (cast `/Game/Blueprints/MichasBlueprints/MovingDoor/BP_NormalDoor` _normal_door))
            (`/Game/Blueprints/MichasBlueprints/MovingDoor/BP_NormalDoor.CloseDoor` _asbp_normal_door_2)
            (else
              (bind _asbp_normal_door_3 (cast `/Game/Blueprints/MichasBlueprints/MovingDoor/BP_NormalDoor` _normal_door))
              (`/Game/Blueprints/MichasBlueprints/MovingDoor/BP_NormalDoor.OpenDoor` _asbp_normal_door_3)))
          (else
            (`KismetSystemLibrary.PrintString` "No Doors Selected")))))))

(fn `UserConstructionScript`)