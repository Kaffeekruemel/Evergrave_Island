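; Floor-style button Blueprint that starts or stops a linked BP_Moving_Platform through box overlaps.
; On overlap, it calls StartMoving(true) if the button's relative Z is at least ButtonMovement, then plays a Timeline that moves the button vertically.
; When overlap ends, the Timeline reverses and StartMoving(false) is sent, unless OneTimeUse keeps the pressed state.
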(event `self.Box.OnComponentBeginOverlap`
  (params (OverlappedComponent :type "PrimitiveComponent Object Reference") (OtherActor :type "Actor Object Reference") (OtherComp :type "PrimitiveComponent Object Reference") (OtherBodyIndex :type Integer) (bFromSweep :type Boolean) (SweepResult :type "HitResult Structure (by ref)"))
  (bind (_relativelocation_x _relativelocation_y _relativelocation_z) (`KismetMathLibrary.BreakVector` (`SceneComponent.RelativeLocation` (`self.button`))))
  (`|ExecutionSequence`
    (:`then_0`
      (if (>= _relativelocation_z (`self.ButtonMovement`))
        (bind _output_get (set `self.ButtonPressed` true))
        (bind _asbp_moving_platform (cast `/Game/Blueprints/MichasBlueprints/MovingPlatform/BP_Moving_Platform` (`self.MovingPlatform`)))
        (`/Game/Blueprints/MichasBlueprints/MovingPlatform/BP_Moving_Platform.StartMoving` _asbp_moving_platform _output_get)))
    (:`then_1`
      (bind (_direction _newtrack_0) (`Timeline|Timeline_0` :!label _label)
        (:`Update`
          (`SceneComponent.K2_SetRelativeLocation` (`self.button`) (`KismetMathLibrary.MakeVector` 0.0 0.0 (* _newtrack_0 (`self.ButtonMovement`))) false false))))))

(event `self.Box.OnComponentEndOverlap`
  (params (OverlappedComponent :type "PrimitiveComponent Object Reference") (OtherActor :type "Actor Object Reference") (OtherComp :type "PrimitiveComponent Object Reference") (OtherBodyIndex :type Integer))
  (`|ExecutionSequence`
    (:`then_0`
      (goto _label :!via `Reverse`))
    (:`then_1`
      (if (not (`self.OneTimeUse`))
        (bind _output_get (set `self.ButtonPressed` false))
        (bind _asbp_moving_platform (cast `/Game/Blueprints/MichasBlueprints/MovingPlatform/BP_Moving_Platform` (`self.MovingPlatform`)))
        (`/Game/Blueprints/MichasBlueprints/MovingPlatform/BP_Moving_Platform.StartMoving` _asbp_moving_platform _output_get)))))

(fn `UserConstructionScript`)