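; BP_OTUBMultiple is a pressable button, filed under moving platform buttons, that sinks when something overlaps its Box and never rises again.
; Each overlap eases the Button component down by ButtonMovement through MoveComponentTo, as long as it sits above a fixed height threshold.
; At or below that threshold it sets ButtonPressed and prints it; this graph does not drive any platform itself.
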(event `self.Box.OnComponentBeginOverlap`
  (params (OverlappedComponent :type "PrimitiveComponent Object Reference") (OtherActor :type "Actor Object Reference") (OtherComp :type "PrimitiveComponent Object Reference") (OtherBodyIndex :type Integer) (bFromSweep :type Boolean) (SweepResult :type "HitResult Structure (by ref)"))
  (bind _button (`self.button`))
  (bind (_relativelocation_x _relativelocation_y _relativelocation_z) (`KismetMathLibrary.BreakVector` (`SceneComponent.RelativeLocation` (`self.button`))))
  (bind (_relativelocation_x_2 _relativelocation_y_2 _relativelocation_z_2) (`KismetMathLibrary.BreakVector` (`SceneComponent.RelativeLocation` (`self.button`))))
  (bind (_relativelocation_x_3 _relativelocation_y_3 _relativelocation_z_3) (`KismetMathLibrary.BreakVector` (`SceneComponent.RelativeLocation` _button)))
  (if (not (>= 10.0 _relativelocation_z))
    (`KismetSystemLibrary.MoveComponentTo` _button (`KismetMathLibrary.MakeVector` _relativelocation_x_3 _relativelocation_y_3 (- _relativelocation_z_3 (`self.ButtonMovement`))) (struct) true false 0.3)
    (if (<= _relativelocation_z_2 10.0)
      (set `self.ButtonPressed` true)
      (`KismetSystemLibrary.PrintString` (`KismetStringLibrary.Conv_BoolToString` (`self.ButtonPressed`))))))

(fn `UserConstructionScript`)