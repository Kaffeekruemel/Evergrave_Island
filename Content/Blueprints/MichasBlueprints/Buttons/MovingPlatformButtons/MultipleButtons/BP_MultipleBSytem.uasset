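; Multi-button puzzle controller that starts a BP_Moving_Platform once all of its assigned buttons, two to five, are pressed.
; BeginPlay prints a warning if either of the two required buttons is missing.
; Every Tick, it casts the buttons along two parallel paths, BP_MTUBMultiple and BP_OTUBMultiple, so all must share one type.
; The filled slots determine which ButtonPressed flags are ANDed before calling StartMoving, which is never called with false.
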(event `self.ReceiveBeginPlay`
  (`|ExecutionSequence`
    (:`then_0`
      (if (not (`KismetSystemLibrary.IsValid` (`self.Button1`)))
        (`KismetSystemLibrary.PrintString` "ButtonOneIsMissing"))
      (if (not (`KismetSystemLibrary.IsValid` (`self.Button2`)))
        (`KismetSystemLibrary.PrintString` "ButtonTwoIsMissing"))
      (if (`KismetSystemLibrary.IsValid` (`self.Button3`))
        (if (`KismetSystemLibrary.IsValid` (`self.Button4`))
          (if (`KismetSystemLibrary.IsValid` (`self.Button5`))
            _))))))

(event `self.ReceiveTick`
  (params (DeltaSeconds :type "Float (single-precision)"))
  (`|ExecutionSequence`
    (:`then_0`
      (if (and (`KismetSystemLibrary.IsValid` (`self.Button1`)) (`KismetSystemLibrary.IsValid` (`self.Button2`)))
        (bind _asbp_mtubmultiple (cast `/Game/Blueprints/MichasBlueprints/Buttons/MovingPlatformButtons/MultipleButtons/BP_MTUBMultiple` (`self.Button1`)))
        (bind _asbp_mtubmultiple_2 (cast `/Game/Blueprints/MichasBlueprints/Buttons/MovingPlatformButtons/MultipleButtons/BP_MTUBMultiple` (`self.Button2`)))
        (if (and (not (`KismetSystemLibrary.IsValid` (`self.Button3`))) (not (`KismetSystemLibrary.IsValid` (`self.Button4`))) (not (`KismetSystemLibrary.IsValid` (`self.Button5`))))
          (bind _asbp_moving_platform (cast `/Game/Blueprints/MichasBlueprints/MovingPlatform/BP_Moving_Platform` (`self.MovingPlatform`)))
          (bind _buttonpressed (`/Game/Blueprints/MichasBlueprints/Buttons/MovingPlatformButtons/MultipleButtons/BP_MTUBMultiple.ButtonPressed` _asbp_mtubmultiple))
          (bind _buttonpressed_2 (`/Game/Blueprints/MichasBlueprints/Buttons/MovingPlatformButtons/MultipleButtons/BP_MTUBMultiple.ButtonPressed` _asbp_mtubmultiple_2))
          (bind _returnvalue (and _buttonpressed _buttonpressed_2))
          (if _returnvalue
            (`/Game/Blueprints/MichasBlueprints/MovingPlatform/BP_Moving_Platform.StartMoving` _asbp_moving_platform _returnvalue))
          (else
            (bind _asbp_mtubmultiple_3 (cast `/Game/Blueprints/MichasBlueprints/Buttons/MovingPlatformButtons/MultipleButtons/BP_MTUBMultiple` (`self.Button3`)))
            (if (and (not (`KismetSystemLibrary.IsValid` (`self.Button4`))) (not (`KismetSystemLibrary.IsValid` (`self.Button5`))))
              (bind _asbp_moving_platform_2 (cast `/Game/Blueprints/MichasBlueprints/MovingPlatform/BP_Moving_Platform` (`self.MovingPlatform`)))
              (bind _buttonpressed_3 (`/Game/Blueprints/MichasBlueprints/Buttons/MovingPlatformButtons/MultipleButtons/BP_MTUBMultiple.ButtonPressed` _asbp_mtubmultiple_3))
              (bind _returnvalue_2 (and _buttonpressed _buttonpressed_2 _buttonpressed_3))
              (if _returnvalue_2
                (`/Game/Blueprints/MichasBlueprints/MovingPlatform/BP_Moving_Platform.StartMoving` _asbp_moving_platform_2 _returnvalue_2))
              (else
                (bind _asbp_mtubmultiple_4 (cast `/Game/Blueprints/MichasBlueprints/Buttons/MovingPlatformButtons/MultipleButtons/BP_MTUBMultiple` (`self.Button4`)))
                (if (not (`KismetSystemLibrary.IsValid` (`self.Button5`)))
                  (bind _asbp_moving_platform_3 (cast `/Game/Blueprints/MichasBlueprints/MovingPlatform/BP_Moving_Platform` (`self.MovingPlatform`)))
                  (bind _buttonpressed_4 (`/Game/Blueprints/MichasBlueprints/Buttons/MovingPlatformButtons/MultipleButtons/BP_MTUBMultiple.ButtonPressed` _asbp_mtubmultiple_4))
                  (bind _returnvalue_3 (and _buttonpressed _buttonpressed_2 _buttonpressed_3 _buttonpressed_4))
                  (if _returnvalue_3
                    (`/Game/Blueprints/MichasBlueprints/MovingPlatform/BP_Moving_Platform.StartMoving` _asbp_moving_platform_3 _returnvalue_3))
                  (else
                    (bind _asbp_mtubmultiple_5 (cast `/Game/Blueprints/MichasBlueprints/Buttons/MovingPlatformButtons/MultipleButtons/BP_MTUBMultiple` (`self.Button5`)))
                    (bind _asbp_moving_platform_4 (cast `/Game/Blueprints/MichasBlueprints/MovingPlatform/BP_Moving_Platform` (`self.MovingPlatform`)))
                    (bind _returnvalue_4 (and _buttonpressed _buttonpressed_2 _buttonpressed_3 _buttonpressed_4 (`/Game/Blueprints/MichasBlueprints/Buttons/MovingPlatformButtons/MultipleButtons/BP_MTUBMultiple.ButtonPressed` _asbp_mtubmultiple_5)))
                    (if _returnvalue_4
                      (`/Game/Blueprints/MichasBlueprints/MovingPlatform/BP_Moving_Platform.StartMoving` _asbp_moving_platform_4 _returnvalue_4))))))))))
    (:`then_1`
      (if (and (`KismetSystemLibrary.IsValid` (`self.Button1`)) (`KismetSystemLibrary.IsValid` (`self.Button2`)))
        (bind _asbp_otubmultiple (cast `/Game/Blueprints/MichasBlueprints/Buttons/MovingPlatformButtons/MultipleButtons/BP_OTUBMultiple` (`self.Button1`)))
        (bind _asbp_otubmultiple_2 (cast `/Game/Blueprints/MichasBlueprints/Buttons/MovingPlatformButtons/MultipleButtons/BP_OTUBMultiple` (`self.Button2`)))
        (if (and (not (`KismetSystemLibrary.IsValid` (`self.Button3`))) (not (`KismetSystemLibrary.IsValid` (`self.Button4`))) (not (`KismetSystemLibrary.IsValid` (`self.Button5`))))
          (bind _asbp_moving_platform_5 (cast `/Game/Blueprints/MichasBlueprints/MovingPlatform/BP_Moving_Platform` (`self.MovingPlatform`)))
          (bind _buttonpressed_5 (`/Game/Blueprints/MichasBlueprints/Buttons/MovingPlatformButtons/MultipleButtons/BP_OTUBMultiple.ButtonPressed` _asbp_otubmultiple))
          (bind _buttonpressed_6 (`/Game/Blueprints/MichasBlueprints/Buttons/MovingPlatformButtons/MultipleButtons/BP_OTUBMultiple.ButtonPressed` _asbp_otubmultiple_2))
          (bind _returnvalue_5 (and _buttonpressed_5 _buttonpressed_6))
          (if _returnvalue_5
            (`/Game/Blueprints/MichasBlueprints/MovingPlatform/BP_Moving_Platform.StartMoving` _asbp_moving_platform_5 _returnvalue_5))
          (else
            (bind _asbp_otubmultiple_3 (cast `/Game/Blueprints/MichasBlueprints/Buttons/MovingPlatformButtons/MultipleButtons/BP_OTUBMultiple` (`self.Button3`)))
            (if (and (not (`KismetSystemLibrary.IsValid` (`self.Button4`))) (not (`KismetSystemLibrary.IsValid` (`self.Button5`))))
              (bind _asbp_moving_platform_6 (cast `/Game/Blueprints/MichasBlueprints/MovingPlatform/BP_Moving_Platform` (`self.MovingPlatform`)))
              (bind _buttonpressed_7 (`/Game/Blueprints/MichasBlueprints/Buttons/MovingPlatformButtons/MultipleButtons/BP_OTUBMultiple.ButtonPressed` _asbp_otubmultiple_3))
              (bind _returnvalue_6 (and _buttonpressed_5 _buttonpressed_6 _buttonpressed_7))
              (if _returnvalue_6
                (`/Game/Blueprints/MichasBlueprints/MovingPlatform/BP_Moving_Platform.StartMoving` _asbp_moving_platform_6 _returnvalue_6))
              (else
                (bind _asbp_otubmultiple_4 (cast `/Game/Blueprints/MichasBlueprints/Buttons/MovingPlatformButtons/MultipleButtons/BP_OTUBMultiple` (`self.Button4`)))
                (if (not (`KismetSystemLibrary.IsValid` (`self.Button5`)))
                  (bind _asbp_moving_platform_7 (cast `/Game/Blueprints/MichasBlueprints/MovingPlatform/BP_Moving_Platform` (`self.MovingPlatform`)))
                  (bind _buttonpressed_8 (`/Game/Blueprints/MichasBlueprints/Buttons/MovingPlatformButtons/MultipleButtons/BP_OTUBMultiple.ButtonPressed` _asbp_otubmultiple_4))
                  (bind _returnvalue_7 (and _buttonpressed_5 _buttonpressed_6 _buttonpressed_7 _buttonpressed_8))
                  (if _returnvalue_7
                    (`/Game/Blueprints/MichasBlueprints/MovingPlatform/BP_Moving_Platform.StartMoving` _asbp_moving_platform_7 _returnvalue_7))
                  (else
                    (bind _asbp_otubmultiple_5 (cast `/Game/Blueprints/MichasBlueprints/Buttons/MovingPlatformButtons/MultipleButtons/BP_OTUBMultiple` (`self.Button5`)))
                    (bind _asbp_moving_platform_8 (cast `/Game/Blueprints/MichasBlueprints/MovingPlatform/BP_Moving_Platform` (`self.MovingPlatform`)))
                    (bind _returnvalue_8 (and _buttonpressed_5 _buttonpressed_6 _buttonpressed_7 _buttonpressed_8 (`/Game/Blueprints/MichasBlueprints/Buttons/MovingPlatformButtons/MultipleButtons/BP_OTUBMultiple.ButtonPressed` _asbp_otubmultiple_5)))
                    (if _returnvalue_8
                      (`/Game/Blueprints/MichasBlueprints/MovingPlatform/BP_Moving_Platform.StartMoving` _asbp_moving_platform_8 _returnvalue_8))))))))))))

(fn `UserConstructionScript`)