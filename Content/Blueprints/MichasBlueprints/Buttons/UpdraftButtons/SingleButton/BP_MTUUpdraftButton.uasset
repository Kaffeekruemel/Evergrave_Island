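; BP_MTUUpdraftButton is a pressure button that controls a referenced Updraft_BP actor while something overlaps its trigger box.
; On overlap, it signals DelayedUpdraft as pressed if the button's relative Z is at or above ButtonMovement, then plays a timeline that moves the button vertically.
; When overlap ends, it reverses the timeline and signals DelayedUpdraft as released.
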(event `self.Box.OnComponentBeginOverlap`
  (params (OverlappedComponent :type "PrimitiveComponent Object Reference") (OtherActor :type "Actor Object Reference") (OtherComp :type "PrimitiveComponent Object Reference") (OtherBodyIndex :type Integer) (bFromSweep :type Boolean) (SweepResult :type "HitResult Structure (by ref)"))
  (bind (_relativelocation_x _relativelocation_y _relativelocation_z) (`KismetMathLibrary.BreakVector` (`SceneComponent.RelativeLocation` (`self.button`))))
  (`|ExecutionSequence`
    (:`then_0`
      (if (<= (`self.ButtonMovement`) _relativelocation_z)
        (bind _output_get (set `self.ButtonPressed` true))
        (bind _asupdraft_bp (cast `/Game/Base/DynamicParaglider/Blueprints/Updraft/Updraft_BP` (`self.Updraft`)))
        (`/Game/Base/DynamicParaglider/Blueprints/Updraft/Updraft_BP.Delayed Updraft` _asupdraft_bp _output_get)))
    (:`then_1`
      (bind (_direction _newtrack_0) (`Timeline|UPDown` :!label _label)
        (:`Update`
          (`SceneComponent.K2_SetRelativeLocation` (`self.button`) (`KismetMathLibrary.MakeVector` 0.0 0.0 (* _newtrack_0 (`self.ButtonMovement`))) false false))))))

(event `self.Box.OnComponentEndOverlap`
  (params (OverlappedComponent :type "PrimitiveComponent Object Reference") (OtherActor :type "Actor Object Reference") (OtherComp :type "PrimitiveComponent Object Reference") (OtherBodyIndex :type Integer))
  (`|ExecutionSequence`
    (:`then_0`
      (goto _label :!via `Reverse`))
    (:`then_1`
      (bind _output_get (set `self.ButtonPressed` false))
      (bind _asupdraft_bp (cast `/Game/Base/DynamicParaglider/Blueprints/Updraft/Updraft_BP` (`self.Updraft`)))
      (`/Game/Base/DynamicParaglider/Blueprints/Updraft/Updraft_BP.Delayed Updraft` _asupdraft_bp _output_get))))

(fn `UserConstructionScript`)