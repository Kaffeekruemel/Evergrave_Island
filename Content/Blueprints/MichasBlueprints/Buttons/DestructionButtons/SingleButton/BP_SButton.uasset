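; BP_SButton is a button actor that destroys a linked Destructable actor once pushed down far enough.
; Each overlap of its Box eases the Button component down by ButtonMovement, as long as it sits above a fixed height threshold.
; At or below that threshold, it sets ButtonPressed and, if Destructable is valid, spawns an explosion emitter at that actor before destroying it.
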(event `self.Box.OnComponentBeginOverlap`
  (params (OverlappedComponent :type "PrimitiveComponent Object Reference") (OtherActor :type "Actor Object Reference") (OtherComp :type "PrimitiveComponent Object Reference") (OtherBodyIndex :type Integer) (bFromSweep :type Boolean) (SweepResult :type "HitResult Structure (by ref)"))
  (bind _destructable (`self.Destructable`))
  (bind _button (`self.button`))
  (bind (_returnvalue_location _returnvalue_rotation _returnvalue_scale) (`KismetMathLibrary.BreakTransform` (`self.GetTransform` _destructable)))
  (bind (_relativelocation_x _relativelocation_y _relativelocation_z) (`KismetMathLibrary.BreakVector` (`SceneComponent.RelativeLocation` _button)))
  (bind (_relativelocation_x_2 _relativelocation_y_2 _relativelocation_z_2) (`KismetMathLibrary.BreakVector` (`SceneComponent.RelativeLocation` (`self.button`))))
  (bind (_relativelocation_x_3 _relativelocation_y_3 _relativelocation_z_3) (`KismetMathLibrary.BreakVector` (`SceneComponent.RelativeLocation` (`self.button`))))
  (if (not (>= 10.0 _relativelocation_z_2))
    (`KismetSystemLibrary.MoveComponentTo` _button (`KismetMathLibrary.MakeVector` _relativelocation_x _relativelocation_y (- _relativelocation_z (`self.ButtonMovement`))) (struct) true false 0.3)
    (if (<= _relativelocation_z_3 10.0)
      (set `self.ButtonPressed` true)
      (if (`KismetSystemLibrary.IsValid` _destructable)
        (`GameplayStatics.SpawnEmitterAtLocation` "/Game/Base/StarterContent/Particles/P_Explosion.P_Explosion" (`self.K2_GetActorLocation` _destructable) (struct) _returnvalue_scale)
        (`self.K2_DestroyActor` (`self.Destructable`))))))

(fn `UserConstructionScript`)