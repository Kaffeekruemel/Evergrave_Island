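; Multi-button puzzle controller that blows up a referenced Destructable actor once all its assigned buttons are pressed.
; Each Tick polls ButtonPressed on two to five BP_MDButton references, with Button1 and Button2 required and the rest optional in slot order.
; When all are pressed, Destroy spawns an explosion at the target's location and scale, then removes it.
; BeginPlay prints a warning if either required button is missing.
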(event `self.ReceiveBeginPlay`
  (`|ExecutionSequence`
    (:`then_0`
      (if (not (`KismetSystemLibrary.IsValid` (`self.Button1`)))
        (`KismetSystemLibrary.PrintString` "ButtonOneIsMissing"))
      (if (not (`KismetSystemLibrary.IsValid` (`self.Button2`)))
        (`KismetSystemLibrary.PrintString` "ButtonTwoIsMissing"))
      (if (`KismetSystemLibrary.IsValid` (`self.Button3`))
        (if (`KismetSystemLibrary.IsValid` (`self.Button4`))
          (if (`KismetSystemLibrary.IsValid` (`self.Button5`))
            _))))))

(event `self.ReceiveTick`
  (params (DeltaSeconds :type "Float (single-precision)"))
  (if (`KismetSystemLibrary.IsValid` (`self.Destructable`))
    (if (and (`KismetSystemLibrary.IsValid` (`self.Button1`)) (`KismetSystemLibrary.IsValid` (`self.Button2`)))
      (bind _asbp_mdbutton (cast `/Game/Blueprints/MichasBlueprints/Buttons/DestructionButtons/MultipleButtons/BP_MDButton` (`self.Button1`)))
      (bind _asbp_mdbutton_2 (cast `/Game/Blueprints/MichasBlueprints/Buttons/DestructionButtons/MultipleButtons/BP_MDButton` (`self.Button2`)))
      (if (and (not (`KismetSystemLibrary.IsValid` (`self.Button3`))) (not (`KismetSystemLibrary.IsValid` (`self.Button4`))) (not (`KismetSystemLibrary.IsValid` (`self.Button5`))))
        (bind _buttonpressed (`/Game/Blueprints/MichasBlueprints/Buttons/DestructionButtons/MultipleButtons/BP_MDButton.ButtonPressed` _asbp_mdbutton))
        (bind _buttonpressed_2 (`/Game/Blueprints/MichasBlueprints/Buttons/DestructionButtons/MultipleButtons/BP_MDButton.ButtonPressed` _asbp_mdbutton_2))
        (if (and _buttonpressed _buttonpressed_2)
          (`self.Destroy`))
        (else
          (bind _asbp_mdbutton_3 (cast `/Game/Blueprints/MichasBlueprints/Buttons/DestructionButtons/MultipleButtons/BP_MDButton` (`self.Button3`)))
          (if (and (not (`KismetSystemLibrary.IsValid` (`self.Button4`))) (not (`KismetSystemLibrary.IsValid` (`self.Button5`))))
            (bind _buttonpressed_3 (`/Game/Blueprints/MichasBlueprints/Buttons/DestructionButtons/MultipleButtons/BP_MDButton.ButtonPressed` _asbp_mdbutton_3))
            (if (and _buttonpressed _buttonpressed_2 _buttonpressed_3)
              (`self.Destroy`))
            (else
              (bind _asbp_mdbutton_4 (cast `/Game/Blueprints/MichasBlueprints/Buttons/DestructionButtons/MultipleButtons/BP_MDButton` (`self.Button4`)))
              (if (not (`KismetSystemLibrary.IsValid` (`self.Button5`)))
                (bind _buttonpressed_4 (`/Game/Blueprints/MichasBlueprints/Buttons/DestructionButtons/MultipleButtons/BP_MDButton.ButtonPressed` _asbp_mdbutton_4))
                (if (and _buttonpressed _buttonpressed_2 _buttonpressed_3 _buttonpressed_4)
                  (`self.Destroy`))
                (else
                  (bind _asbp_mdbutton_5 (cast `/Game/Blueprints/MichasBlueprints/Buttons/DestructionButtons/MultipleButtons/BP_MDButton` (`self.Button5`)))
                  (if (and _buttonpressed _buttonpressed_2 _buttonpressed_3 _buttonpressed_4 (`/Game/Blueprints/MichasBlueprints/Buttons/DestructionButtons/MultipleButtons/BP_MDButton.ButtonPressed` _asbp_mdbutton_5))
                    (`self.Destroy`)))))))))))

(event `Destroy`
  (bind _destructable (`self.Destructable`))
  (bind (_returnvalue_location _returnvalue_rotation _returnvalue_scale) (`KismetMathLibrary.BreakTransform` (`self.GetTransform` _destructable)))
  (`GameplayStatics.SpawnEmitterAtLocation` "/Game/Base/StarterContent/Particles/P_Explosion.P_Explosion" (`self.K2_GetActorLocation` _destructable) (struct) _returnvalue_scale)
  (`self.K2_DestroyActor` (`self.Destructable`)))

(fn `UserConstructionScript`)