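; BP_Cable is a spline-built cable with an enable state, able to depend on up to three linked side cables.
; The construction script lays spline meshes in segments sized by actor Z scale.
; Seitencable sets Enable, and Tick polls it or the linked cables' states to spawn steam at spline points every frame.
; The segment array fill is disconnected, so the side-cable steam loop and single-cable green material lack valid segments.
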(event Custom|Seitencable
  (params (Enable :type Boolean))
  (Variables|Default|SetEnable Enable))

(event Collision|EventActorBeginOverlap
  (params (OtherActor :type Actor%20Object%20Reference)))

(event EventTick
  (params (DeltaSeconds :type Float%20%28single-precision%29))
  (if (Variables|Default|GetSidecable)
    (if (Variables|Default|GetEnable)
      (for _array_element (Variables|Default|GetSplineComponentArray)
        (Effects|SpawnEmitteratLocation "/Game/Base/StarterContent/Particles/P_Steam_Lit.P_Steam_Lit" (Spline|GetLocationatSplinePoint (Variables|Default|GetSpline) 0 "World"))))
    (elif (Variables|Default|GetSinglecable)
      (if (Variables|Default|GetEnable)
        (Rendering|Material|SetMaterial (stale _array_element) (stale _array_index) "/Game/M_Cape_Green.M_Cape_Green"))
      (elif (Math|Boolean|ANDBoolean (Utilities|IsValid (Variables|Default|GetSidecable1)) (not (Utilities|IsValid (Variables|Default|GetSidecable2))) (not (Utilities|IsValid (Variables|Default|GetSidecable3))))
        (bind _asbp_cable (Utilities|Casting|CastToBP_Cable (Variables|Default|GetSidecable1)))
        (if (Variables|BP_Cable_C|GetEnable _asbp_cable)
          (Effects|SpawnEmitteratLocation "/Game/Base/StarterContent/Particles/P_Steam_Lit.P_Steam_Lit" (Spline|GetLocationatSplinePoint (Variables|Default|GetSpline) 0 "World")))
        (elif (Math|Boolean|ANDBoolean (Utilities|IsValid (Variables|Default|GetSidecable1)) (Utilities|IsValid (Variables|Default|GetSidecable2)) (not (Utilities|IsValid (Variables|Default|GetSidecable3))))
          (bind _asbp_cable_2 (Utilities|Casting|CastToBP_Cable (Variables|Default|GetSidecable1)))
          (bind _asbp_cable_3 (Utilities|Casting|CastToBP_Cable (Variables|Default|GetSidecable2)))
          (if (and (Variables|BP_Cable_C|GetEnable _asbp_cable_2) (Variables|BP_Cable_C|GetEnable _asbp_cable_3))
            (Effects|SpawnEmitteratLocation "/Game/Base/StarterContent/Particles/P_Steam_Lit.P_Steam_Lit" (Spline|GetLocationatSplinePoint (Variables|Default|GetSpline) 1 "World")))
          (elif (Math|Boolean|ANDBoolean (Utilities|IsValid (Variables|Default|GetSidecable1)) (Utilities|IsValid (Variables|Default|GetSidecable2)) (Utilities|IsValid (Variables|Default|GetSidecable3)))
            (bind _asbp_cable_4 (Utilities|Casting|CastToBP_Cable (Variables|Default|GetSidecable1)))
            (bind _asbp_cable_5 (Utilities|Casting|CastToBP_Cable (Variables|Default|GetSidecable2)))
            (bind _asbp_cable_6 (Utilities|Casting|CastToBP_Cable (Variables|Default|GetSidecable3)))
            (if (Math|Boolean|ANDBoolean (Variables|BP_Cable_C|GetEnable _asbp_cable_4) (Variables|BP_Cable_C|GetEnable _asbp_cable_5) (Variables|BP_Cable_C|GetEnable _asbp_cable_6))
              (Effects|SpawnEmitteratLocation "/Game/Base/StarterContent/Particles/P_Steam_Lit.P_Steam_Lit" (Spline|GetLocationatSplinePoint (Variables|Default|GetSpline) 2 "World")))
            (elif (Utilities|IsValid (Variables|Default|GetSidecable1))
              _)))))))

(fn ConstructionScript
  (bind _spline (Variables|Default|GetSpline))
  (bind _spline_2 (Variables|Default|GetSpline))
  (Variables|Default|SetSectionLenght (* (.z (Transformation|GetActorScale3D)) 1e+02))
  (for _index (range 0 (- (Math|Float|Truncate (/ (Spline|GetSplineLength (Variables|Default|GetSpline)) (Variables|Default|GetSectionLenght))) 1))
    (bind _returnvalue (AddComponent|AddSplineMeshComponent false))
    (Variables|Default|SetMesh _returnvalue)
    (SplineMesh|SetForwardAxis _returnvalue "Z" true)
    (Collision|SetCollisionEnabled _returnvalue "QueryAndPhysics")
    (SplineMesh|SetStartandEnd _returnvalue (Spline|GetLocationatDistanceAlongSpline _spline (* _index (Variables|Default|GetSectionLenght)) "Local") (Math|Vector|ClampVectorSize (Spline|GetTangentatDistanceAlongSpline _spline (* _index (Variables|Default|GetSectionLenght)) "Local") 0.0 (Variables|Default|GetSectionLenght)) (Spline|GetLocationatDistanceAlongSpline _spline_2 (* (+ _index 1) (Variables|Default|GetSectionLenght)) "Local") (Math|Vector|ClampVectorSize (Spline|GetTangentatDistanceAlongSpline _spline_2 (* (+ _index 1) (Variables|Default|GetSectionLenght)) "Local") 0.0 (Variables|Default|GetSectionLenght)) true :!class /Script/Engine.SplineMeshComponent)))